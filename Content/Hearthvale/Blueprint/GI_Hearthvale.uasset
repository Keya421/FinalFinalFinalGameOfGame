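; Game instance for Hearthvale that carries player, restaurant and world state across levels and handles saving and loading.
; Save and load copy that state through SG_Hearthvale in hard-coded slot "1"; Init applies user settings and saved audio volumes.
; CacheFurniture snapshots restaurant decor and pickups into structs, with table, chair and chest data.
; OpenLevel stores furniture, inventory and time before travel; DisplayTutoriala builds data-table tutorial widgets and records seen ones.
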(event `LoadSave`
  (params (Slot :type String))
  (bind _returnvalue (`GameplayStatics.DoesSaveGameExist` "1"))
  (if _returnvalue
    (bind _returnvalue_2 (`GameplayStatics.LoadGameFromSlot` "1"))
    (bind _assg_hearthvale (cast `/Game/Hearthvale/Blueprint/SG_Hearthvale` _returnvalue_2))
    (set `self.Inventory` (`/Game/Hearthvale/Blueprint/SG_Hearthvale.InventorySave` _assg_hearthvale))
    (set `self.LoadedFurniture` (`/Game/Hearthvale/Blueprint/SG_Hearthvale.SavedToGameFurniture` _assg_hearthvale))
    (set `self.AllOrders` (`/Game/Hearthvale/Blueprint/SG_Hearthvale.AllOrders` _assg_hearthvale))
    (set `self.PlayerMoney` (`/Game/Hearthvale/Blueprint/SG_Hearthvale.PlayerMoney` _assg_hearthvale))
    (set `self.PlayerAllTimeMoney` (`/Game/Hearthvale/Blueprint/SG_Hearthvale.PlayerAllTimeMoney` _assg_hearthvale))
    (set `self.PlayerUnlockedRecipes` (`/Game/Hearthvale/Blueprint/SG_Hearthvale.PlayerUnlockedRecipes` _assg_hearthvale))
    (set `self.bVendorQuestFinished` (`/Game/Hearthvale/Blueprint/SG_Hearthvale.bIsVendorQuestFinished` _assg_hearthvale))
    (set `self.TutorialList` (`/Game/Hearthvale/Blueprint/SG_Hearthvale.TutorialList` _assg_hearthvale))
    (set `self.WorldTime` (`/Game/Hearthvale/Blueprint/SG_Hearthvale.WorldTime` _assg_hearthvale))
    (set `self.PlayerStepCount` (`/Game/Hearthvale/Blueprint/SG_Hearthvale.PlayerStepCount` _assg_hearthvale))
    (`self.OpenLevel` "/Game/Hearthvale/GameMap/Levels/RestaurantLevel.RestaurantLevel")
    (else
      (`KismetSystemLibrary.PrintString` "Save Doesnt exist")
      (`GameplayStatics.OpenLevelBySoftObjectPtr` "/Game/Hearthvale/GameMap/Levels/RestaurantLevel.RestaurantLevel"))))

(event `SaveGame`
  (params (Slot :type String))
  (bind _asbp_third_person_character (cast `/Game/ThirdPerson/Blueprints/BP_ThirdPersonCharacter` (`GameplayStatics.GetPlayerPawn` 0) :!pure true))
  (bind _returnvalue (`GameplayStatics.CreateSaveGameObject` "/Game/Hearthvale/Blueprint/SG_Hearthvale.SG_Hearthvale_C"))
  (set `/Game/Hearthvale/Blueprint/SG_Hearthvale.PlayerStepCount` (`self.PlayerStepCount`) _returnvalue)
  (set `/Game/Hearthvale/Blueprint/SG_Hearthvale.InventorySave` (`self.Inventory`) _returnvalue)
  (set `/Game/Hearthvale/Blueprint/SG_Hearthvale.SavedToGameFurniture` (`self.LoadedFurniture`) _returnvalue)
  (set `/Game/Hearthvale/Blueprint/SG_Hearthvale.AllOrders` (`self.AllOrders`) _returnvalue)
  (set `/Game/Hearthvale/Blueprint/SG_Hearthvale.PlayerMoney` (`self.PlayerMoney`) _returnvalue)
  (set `/Game/Hearthvale/Blueprint/SG_Hearthvale.PlayerAllTimeMoney` (`self.PlayerAllTimeMoney`) _returnvalue)
  (set `/Game/Hearthvale/Blueprint/SG_Hearthvale.PlayerUnlockedRecipes` (`self.PlayerUnlockedRecipes`) _returnvalue)
  (set `/Game/Hearthvale/Blueprint/SG_Hearthvale.bIsVendorQuestFinished` (`self.bVendorQuestFinished`) _returnvalue)
  (set `/Game/Hearthvale/Blueprint/SG_Hearthvale.TutorialList` (`self.TutorialList`) _returnvalue)
  (bind _returnvalue_2 (`GameplayStatics.GetActorOfClass` "/Game/Hearthvale/Blueprint/Weather/BP_WeatherSpawn.BP_WeatherSpawn_C"))
  (`/Engine/EditorBlueprintResources/StandardMacros.IsValid` _returnvalue_2
    (:`Is Valid`
      (set `self.WorldTime` (`/Game/Hearthvale/Blueprint/Weather/BP_WeatherSpawn.Time` _returnvalue_2)))
    (:`Is Not Valid`
      _))
  (set `/Game/Hearthvale/Blueprint/SG_Hearthvale.WorldTime` (`self.WorldTime`) _returnvalue)
  (`GameplayStatics.SaveGameToSlot` _returnvalue "1")
  (`/Game/ThirdPerson/Blueprints/BP_ThirdPersonCharacter.StartDialogue` _asbp_third_person_character (`|MakeArray` (make `/Game/Hearthvale/Blueprint/UI/Dialogue/ST_DialogueOptions` "Successfully saved." 1) (make `/Game/Hearthvale/Blueprint/UI/Dialogue/ST_DialogueOptions` "See you next time!" 0 null _ true) :!type "/Game/Hearthvale/Blueprint/UI/Dialogue/ST_DialogueOptions Structure"))
  (add `/Game/Hearthvale/A/UI-AP/DialogueTest.OnFinishDialogue` (`/Game/ThirdPerson/Blueprints/BP_ThirdPersonCharacter.DialogueWidget` _asbp_third_person_character) (delegate `QuitGame`)))

(event `QuitGame`
  (`GameplayStatics.OpenLevelBySoftObjectPtr` "/Game/Hearthvale/GameMap/Levels/MainMenuMap.MainMenuMap"))

(event `self.ReceiveInit`
  (bind _returnvalue (`GameUserSettings.GetGameUserSettings`))
  (`GameUserSettings.LoadSettings` _returnvalue false)
  (`GameUserSettings.ApplySettings` _returnvalue true)
  (bind _returnvalue_2 (`GameplayStatics.DoesSaveGameExist` "settings"))
  (if _returnvalue_2
    (bind _returnvalue_3 (`GameplayStatics.LoadGameFromSlot` "settings"))
    (bind _assg_hearthvale (cast `/Game/Hearthvale/Blueprint/SG_Hearthvale` _returnvalue_3))
    (bind _output_get (set `self.PlayerSettings` (`/Game/Hearthvale/Blueprint/SG_Hearthvale.PlayerSettings` _assg_hearthvale)))
    (bind (_advancedquit _audiosettings) (break `/Game/Hearthvale/Blueprint/PlayerData/ST_PlayerSettings` _output_get))
    (`GameplayStatics.SetSoundMixClassOverride` "/Game/Hearthvale/A/SOUNDS-AP/MasterVolume.MasterVolume" "/Engine/EngineSounds/Music.Music" (`.MusicVolume_6_96B3FE8C47BBCBDDA135B3B7F346A0A2` (break `/Game/Hearthvale/Blueprint/PlayerData/ST_PlayerAudioSettings` _audiosettings)) 1.0 0.5)
    (`GameplayStatics.SetSoundMixClassOverride` "/Game/Hearthvale/A/SOUNDS-AP/MasterVolume.MasterVolume" "/Engine/EngineSounds/SFX.SFX" (`.SFXVolume_7_E51952914280E82BDB1C13A8FB3C974E` (break `/Game/Hearthvale/Blueprint/PlayerData/ST_PlayerAudioSettings` _audiosettings)) 1.0 0.5)
    (`GameplayStatics.SetSoundMixClassOverride` "/Game/Hearthvale/A/SOUNDS-AP/MasterVolume.MasterVolume" "/Engine/EngineSounds/Voice.Voice" (`.VoiceVolume_8_7B0F2B154476D39B7B214F989AD50F12` (break `/Game/Hearthvale/Blueprint/PlayerData/ST_PlayerAudioSettings` _audiosettings)) 1.0 0.5)
    (`GameplayStatics.SetSoundMixClassOverride` "/Game/Hearthvale/A/SOUNDS-AP/MasterVolume.MasterVolume" "/Engine/EngineSounds/Master.Master" (break `/Game/Hearthvale/Blueprint/PlayerData/ST_PlayerAudioSettings` _audiosettings) 1.0 0.5)
    (`GameplayStatics.PushSoundMixModifier` "/Game/Hearthvale/A/SOUNDS-AP/MasterVolume.MasterVolume")))

(fn `CacheFurniture`
  (locals (SaveFurnitureArray :type "Array of /Game/Hearthvale/Blueprint/Restaurant/Saving/ST_FurnitureSave Structure") (StorageItems :type "Array of /Game/Kristian/inventory/ST_GIItems Structure"))
  (bind _savefurniturearray (`local.SaveFurnitureArray`))
  (bind _storageitems (`local.StorageItems`))
  (bind _returnvalue (`GameplayStatics.GetCurrentLevelName` true))
  (if (`KismetStringLibrary.EqualEqual_StrStr` _returnvalue "RestaurantLevel")
    (bind _outactors (`GameplayStatics.GetAllActorsOfClass` "/Game/Hearthvale/Blueprint/Restaurant/Actors/BP_RestaurantDecor.BP_RestaurantDecor_C"))
    (for _array_element _outactors
      (bind _returnvalue_2 (`GameplayStatics.GetObjectClass` _array_element))
      (if (`KismetMathLibrary.ClassIsChildOf` _returnvalue_2 "/Game/Hearthvale/Blueprint/Restaurant/Actors/Furniture/Seating/zParentClasses/BP_TableParent.BP_TableParent_C")
        (`KismetSystemLibrary.PrintString` "Table")
        (bind _asbp_table_parent (cast `/Game/Hearthvale/Blueprint/Restaurant/Actors/Furniture/Seating/zParentClasses/BP_TableParent` _array_element :!pure true))
        (bind _dataasset (`/Game/Hearthvale/Blueprint/Restaurant/Actors/BP_RestaurantDecor.DataAsset` _array_element))
        (`KismetArrayLibrary.Array_Add` (`local.SaveFurnitureArray`) (make `/Game/Hearthvale/Blueprint/Restaurant/Saving/ST_FurnitureSave` (`GameplayStatics.GetObjectClass` _asbp_table_parent) (`Actor.GetTransform` _asbp_table_parent) (`/Game/Hearthvale/Blueprint/Restaurant/Actors/BP_RestaurantDecor.Width` _asbp_table_parent) (`/Game/Hearthvale/Blueprint/Restaurant/Actors/BP_RestaurantDecor.Length` _asbp_table_parent) (struct) (make `/Game/Hearthvale/Blueprint/Restaurant/Saving/ST_SaveTable` (`/Game/Hearthvale/Blueprint/Restaurant/Actors/Furniture/Seating/zParentClasses/BP_TableParent.AssignedOrder` _asbp_table_parent) (`/Game/Hearthvale/Blueprint/Restaurant/Actors/Furniture/Seating/zParentClasses/BP_TableParent.isTableNotTaken` _asbp_table_parent) true) (struct) (struct) _dataasset))
        (elif (`KismetMathLibrary.ClassIsChildOf` _returnvalue_2 "/Game/Hearthvale/Blueprint/Restaurant/Actors/Furniture/Seating/zParentClasses/BP_ChairParent.BP_ChairParent_C")
          (`KismetSystemLibrary.PrintString` "Chair")
          (bind _asbp_chair_parent (cast `/Game/Hearthvale/Blueprint/Restaurant/Actors/Furniture/Seating/zParentClasses/BP_ChairParent` _array_element :!pure true))
          (bind _assignedcustomer (`/Game/Hearthvale/Blueprint/Restaurant/Actors/Furniture/Seating/zParentClasses/BP_ChairParent.AssignedCustomer` _asbp_chair_parent))
          (bind _returnvalue_3 (`KismetSystemLibrary.IsValid` _assignedcustomer))
          (if _returnvalue_3
            (bind _returnvalue_4 (`GameplayStatics.GetObjectClass` _asbp_chair_parent))
            (bind _returnvalue_5 (`Actor.GetTransform` _asbp_chair_parent))
            (bind _width (`/Game/Hearthvale/Blueprint/Restaurant/Actors/BP_RestaurantDecor.Width` _asbp_chair_parent))
            (bind _length (`/Game/Hearthvale/Blueprint/Restaurant/Actors/BP_RestaurantDecor.Length` _asbp_chair_parent))
            (`KismetArrayLibrary.Array_Add` _savefurniturearray (make `/Game/Hearthvale/Blueprint/Restaurant/Saving/ST_FurnitureSave` _returnvalue_4 _returnvalue_5 _width _length (make `/Game/Hearthvale/Blueprint/Restaurant/Saving/ST_SaveChair` _returnvalue_3 (`|ConvertAsset` (`/Game/Hearthvale/Blueprint/Restaurant/Actors/Customer/BP_SingleCustomer.CustomerTexture` _assignedcustomer)) true) (struct :`AssignedOrder` "(())") (struct) (struct) _dataasset))
            (else
              (`KismetArrayLibrary.Array_Add` _savefurniturearray (make `/Game/Hearthvale/Blueprint/Restaurant/Saving/ST_FurnitureSave` _returnvalue_4 _returnvalue_5 _width _length (make `/Game/Hearthvale/Blueprint/Restaurant/Saving/ST_SaveChair` _returnvalue_3 null true) (struct :`AssignedOrder` "(())") (struct) (struct) _dataasset))))
          (elif (== _returnvalue_2 "/Game/Hearthvale/Blueprint/Restaurant/Actors/Furniture/Other/BP_StorageChest.BP_StorageChest_C")
            (bind _asbp_storage_chest (cast `/Game/Hearthvale/Blueprint/Restaurant/Actors/Furniture/Other/BP_StorageChest` _array_element))
            (for _array_element_2 (`/Game/Hearthvale/Blueprint/Restaurant/Actors/Furniture/Other/BP_StorageChest.chestStorage` _asbp_storage_chest)
              (bind _returnvalue_6 (`GameplayStatics.GetObjectClass` (break `/Game/Kristian/inventory/ST_items` _array_element_2)))
              (if (== _returnvalue_6 "/Game/Hearthvale/Blueprint/Items/ItemData/Food/DA_ItemFood.DA_ItemFood_C")
                (bind _asda_item_food (cast `/Game/Hearthvale/Blueprint/Items/ItemData/Food/DA_ItemFood` (break `/Game/Kristian/inventory/ST_items` _array_element_2) :!pure true))
                (`KismetArrayLibrary.Array_Add` _storageitems (make `/Game/Kristian/inventory/ST_GIItems` "/Game/Hearthvale/Blueprint/Items/ItemData/Food/DA_ItemFood.DA_ItemFood_C" (`.ItemAmount_23_988A17D64E15A30C67E07FA90A341A42` (break `/Game/Kristian/inventory/ST_items` _array_element_2)) (make `/Game/Kristian/inventory/ST_GIDishData` (`/Game/Hearthvale/Blueprint/Items/ItemData/DA_Item.ItemName` _asda_item_food) (`/Game/Hearthvale/Blueprint/Items/ItemData/Food/DA_ItemFood.DishAttributes` _asda_item_food) (`|ConvertAsset` (`/Game/Hearthvale/Blueprint/Items/ItemData/DA_Item.ItemIcon` _asda_item_food)))))
                (elif (`KismetSystemLibrary.IsValidClass` _returnvalue_6)
                  (`KismetArrayLibrary.Array_Add` _storageitems (make `/Game/Kristian/inventory/ST_GIItems` _returnvalue_6 (`.ItemAmount_23_988A17D64E15A30C67E07FA90A341A42` (break `/Game/Kristian/inventory/ST_items` _array_element_2))))
                  (else
                    (`KismetArrayLibrary.Array_Add` _storageitems)))))
            (`KismetArrayLibrary.Array_Add` (`local.SaveFurnitureArray`) (make `/Game/Hearthvale/Blueprint/Restaurant/Saving/ST_FurnitureSave` (`GameplayStatics.GetObjectClass` _asbp_storage_chest) (`Actor.GetTransform` _asbp_storage_chest) (`/Game/Hearthvale/Blueprint/Restaurant/Actors/BP_RestaurantDecor.Width` _asbp_storage_chest) (`/Game/Hearthvale/Blueprint/Restaurant/Actors/BP_RestaurantDecor.Length` _asbp_storage_chest) (struct) (struct :`AssignedOrder` "(())") (struct) (make `/Game/Hearthvale/Blueprint/Restaurant/Saving/ST_SaveStorage` (`local.StorageItems`) true) _dataasset))
            (`KismetArrayLibrary.Array_Clear` (`local.StorageItems`))
            (else
              (`KismetSystemLibrary.PrintString` "Everything Else")
              (`KismetArrayLibrary.Array_Add` (`local.SaveFurnitureArray`) (make `/Game/Hearthvale/Blueprint/Restaurant/Saving/ST_FurnitureSave` (`GameplayStatics.GetObjectClass` _array_element) (`Actor.GetTransform` _array_element) (`/Game/Hearthvale/Blueprint/Restaurant/Actors/BP_RestaurantDecor.Width` _array_element) (`/Game/Hearthvale/Blueprint/Restaurant/Actors/BP_RestaurantDecor.Length` _array_element) (struct) (struct :`AssignedOrder` "(())") (struct) (struct) _dataasset)))))))
    (bind _outactors_2 (`GameplayStatics.GetAllActorsOfClass` "/Game/Hearthvale/Blueprint/Items/Blueprints/BP_ItemPickup.BP_ItemPickup_C"))
    (for _array_element_3 _outactors_2
      (`KismetArrayLibrary.Array_Add` (`local.SaveFurnitureArray`) (make `/Game/Hearthvale/Blueprint/Restaurant/Saving/ST_FurnitureSave` (`GameplayStatics.GetObjectClass` _array_element_3) (`Actor.GetTransform` _array_element_3) 0 0 (struct) (struct :`AssignedOrder` "(())") (make `/Game/Hearthvale/Blueprint/Restaurant/Saving/ST_ItemDropSave` (`/Game/Hearthvale/Blueprint/Items/Blueprints/BP_ItemPickup.Item` _array_element_3) (`/Game/Hearthvale/Blueprint/Items/Blueprints/BP_ItemPickup.ItemCount` _array_element_3) true))))
    (set `self.LoadedFurniture` (`local.SaveFurnitureArray`))
    (`KismetSystemLibrary.PrintString` "Cached Furniture")
    (else
      (`KismetSystemLibrary.RaiseScriptError` "Cannot save Furniture, not in RestaurantLevel map."))))

(fn `DisplayTutoriala`
  (params (`SetWidget?` :type Boolean) (`Row Name` :type Name) (`IsPlayerBook?` :type Boolean))
  (returns (TutorialWidget :type "/Game/Hearthvale/Blueprint/UI/Tutorial/WBP_PlayerTutorial Object Reference"))
  (locals (NewLocalVar :type Boolean))
  (bind _returnvalue (`GameplayStatics.GetPlayerController` 0))
  (bind _tutoriallist (`self.TutorialList`))
  (bind _asbp_third_person_character (cast `/Game/ThirdPerson/Blueprints/BP_ThirdPersonCharacter` (`Controller.K2_GetPawn` _returnvalue) :!pure true))
  (if `IsPlayerBook?`
    (bind _returnvalue_2 (`|GetDataTableRow` "/Game/Hearthvale/Blueprint/UI/Tutorial/AllTutorials/DT_TutorialTable.DT_TutorialTable" `Row Name` :!label _label)
      (:`then`
        (bind _returnvalue_3 (`|CreateWidget` "/Game/Hearthvale/Blueprint/UI/Tutorial/WBP_PlayerTutorial.WBP_PlayerTutorial_C" _returnvalue))
        (bind (_title _description _texturearray _fps _numofframes) (break `/Game/Hearthvale/Blueprint/UI/Tutorial/AllTutorials/ST_TutorialOptions` _returnvalue_2))
        (set `/Game/Hearthvale/Blueprint/UI/Tutorial/WBP_PlayerTutorial.Title` _title _returnvalue_3)
        (set `/Game/Hearthvale/Blueprint/UI/Tutorial/WBP_PlayerTutorial.Description` _description _returnvalue_3)
        (set `/Game/Hearthvale/Blueprint/UI/Tutorial/WBP_PlayerTutorial.GIF` _texturearray _returnvalue_3)
        (set `/Game/Hearthvale/Blueprint/UI/Tutorial/WBP_PlayerTutorial.FPS` _fps _returnvalue_3)
        (set `/Game/Hearthvale/Blueprint/UI/Tutorial/WBP_PlayerTutorial.FrameCount` _numofframes _returnvalue_3)
        (if (not (not `SetWidget?`))
          (`UserWidget.AddToViewport` _returnvalue_3 0)
          (`/Game/ThirdPerson/Blueprints/BP_ThirdPersonCharacter.EnableShowMouse` _asbp_third_person_character true)
          (`/Game/ThirdPerson/Blueprints/BP_ThirdPersonCharacter.EnableMovement` _asbp_third_person_character false))
        (for (_array_element _array_index) _tutoriallist
          (bind (_seen_ _rowname) (break `/Game/Hearthvale/Blueprint/PlayerData/ST_ShownTutorialOption` _array_element))
          (if (== `Row Name` _rowname)
            (`KismetArrayLibrary.Array_Set` _tutoriallist _array_index (make `/Game/Hearthvale/Blueprint/PlayerData/ST_ShownTutorialOption` true _rowname))
            (set `local.NewLocalVar` true)))
        (if (not (`local.NewLocalVar`))
          (`KismetArrayLibrary.Array_Add` _tutoriallist (make `/Game/Hearthvale/Blueprint/PlayerData/ST_ShownTutorialOption` true `Row Name`)))
        (return _returnvalue_3))
      (:`RowNotFound`
        (`KismetSystemLibrary.RaiseScriptError` (`KismetStringLibrary.Concat_StrStr` "Row \"" (`KismetStringLibrary.Conv_NameToString` `Row Name`) "\" is NOT valid"))))
    (elif (== (`KismetArrayLibrary.Array_Find` (`self.TutorialList`) (make `/Game/Hearthvale/Blueprint/PlayerData/ST_ShownTutorialOption` true `Row Name`)) -1)
      (goto _label))))

(fn `LoadPlayerSettings`
  (bind (_playersettings_advancedquit _playersettings_audiosettings) (break `/Game/Hearthvale/Blueprint/PlayerData/ST_PlayerSettings` (`self.PlayerSettings`)))
  (bind (_mastervolume _musicvolume _sfxvolume _voicevolume) (break `/Game/Hearthvale/Blueprint/PlayerData/ST_PlayerAudioSettings` _playersettings_audiosettings))
  (`GameplayStatics.SetSoundMixClassOverride` "/Game/Hearthvale/A/SOUNDS-AP/MasterVolume.MasterVolume" "/Engine/EngineSounds/Music.Music" _musicvolume 1.0 0.0)
  (`GameplayStatics.SetSoundMixClassOverride` "/Game/Hearthvale/A/SOUNDS-AP/MasterVolume.MasterVolume" "/Engine/EngineSounds/SFX.SFX" _sfxvolume 1.0 0.0)
  (`GameplayStatics.SetSoundMixClassOverride` "/Game/Hearthvale/A/SOUNDS-AP/MasterVolume.MasterVolume" "/Engine/EngineSounds/Voice.Voice" _voicevolume 1.0 0.0)
  (`GameplayStatics.SetSoundMixClassOverride` "/Game/Hearthvale/A/SOUNDS-AP/MasterVolume.MasterVolume" "/Engine/EngineSounds/Master.Master" _mastervolume 1.0 0.0)
  (`GameplayStatics.PushSoundMixModifier` "/Game/Hearthvale/A/SOUNDS-AP/MasterVolume.MasterVolume"))

(fn `OpenLevel`
  (params (Level :type "World Soft Object Reference"))
  (bind _asbp_third_person_character (cast `/Game/ThirdPerson/Blueprints/BP_ThirdPersonCharacter` (`GameplayStatics.GetPlayerPawn` 0) :!pure true))
  (bind _returnvalue (`GameplayStatics.GetActorOfClass` "/Game/Hearthvale/Blueprint/Restaurant/BP_RestaurantLogic.BP_RestaurantLogic_C"))
  (`/Engine/EditorBlueprintResources/StandardMacros.IsValid` _returnvalue
    (:`Is Valid`
      (`/Game/Hearthvale/Blueprint/Restaurant/BP_RestaurantLogic.SaveFurniture` _returnvalue))
    (:`Is Not Valid`
      _))
  (`/Engine/EditorBlueprintResources/StandardMacros.IsValid` _asbp_third_person_character
    (:`Is Valid`
      (`/Game/ThirdPerson/Blueprints/BP_ThirdPersonCharacter.SaveInventory_GI` _asbp_third_person_character))
    (:`Is Not Valid`
      _))
  (bind _returnvalue_2 (`GameplayStatics.GetActorOfClass` "/Game/Hearthvale/Blueprint/Weather/BP_WeatherSpawn.BP_WeatherSpawn_C"))
  (`/Engine/EditorBlueprintResources/StandardMacros.IsValid` _returnvalue_2
    (:`Is Valid`
      (set `self.WorldTime` (`/Game/Hearthvale/Blueprint/Weather/BP_WeatherSpawn.Time` _returnvalue_2)))
    (:`Is Not Valid`
      _))
  (`GameplayStatics.OpenLevelBySoftObjectPtr` Level))

(fn `SavePlayerSettings`
  (locals (SelectedSave :type "/Game/Hearthvale/Blueprint/SG_Hearthvale Object Reference"))
  (bind _returnvalue (`GameUserSettings.GetGameUserSettings`))
  (`GameUserSettings.SaveSettings` _returnvalue))