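; Base Blueprint for choppable trees that yield wood when the player interacts with them.
; Interact checks that the item in the player's selected hotbar slot is BP_ForageAxe, then passes a point just ahead of the player's Arrow1 to DropWood.
; DropWood spawns a BP_ItemPickup there holding a single WoodItem and destroys the tree at once.
; An unconnected offset calculation relative to the tree remains in DropWood.
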(event `/Game/Hearthvale/Blueprint/PlayerData/BPI_Interact.Interact`
  (bind _asbp_third_person_character (cast `/Game/ThirdPerson/Blueprints/BP_ThirdPersonCharacter` (`GameplayStatics.GetPlayerPawn` 0) :!pure true))
  (if (== (`GameplayStatics.GetObjectClass` (`.ItemClass_27_04EDF3F8416E8B472A41CC8E06E4FB6F` (break `/Game/Kristian/inventory/ST_items` (`/Game/Kristian/inventory/WBP_ItemSlot.itemData` (`|GetArrayItem` (`/Game/Kristian/inventory/WBP_inventory.HotbarArray` (`/Game/ThirdPerson/Blueprints/BP_ThirdPersonCharacter.InventoryWidget` _asbp_third_person_character)) (- (`/Game/ThirdPerson/Blueprints/BP_ThirdPersonCharacter.SelectedSlot` _asbp_third_person_character) 1)))))) "/Game/Hearthvale/Blueprint/Items/ItemData/Tools/ToolsData/BP_ForageAxe.BP_ForageAxe_C")
    (`self.DropWood` (+ (* (`SceneComponent.GetForwardVector` (`/Game/ThirdPerson/Blueprints/BP_ThirdPersonCharacter.Arrow1` _asbp_third_person_character)) 100.0) (`self.K2_GetActorLocation` _asbp_third_person_character)))))

(fn `DropWood`
  (params (`Hit Location` :type "Vector Structure"))
  (bind _returnvalue (`|SpawnActorFromClass` "/Game/Hearthvale/Blueprint/Items/Blueprints/BP_ItemPickup.BP_ItemPickup_C" (`KismetMathLibrary.MakeTransform` (`KismetMathLibrary.MakeVector` `Hit Location_X` `Hit Location_Y` `Hit Location_Z`)) "Undefined" "MultiplyWithRoot" null null))
  (set `/Game/Hearthvale/Blueprint/Items/Blueprints/BP_ItemPickup.Item` (`self.WoodItem`) _returnvalue)
  (set `/Game/Hearthvale/Blueprint/Items/Blueprints/BP_ItemPickup.ItemCount` 1 _returnvalue)
  (`self.K2_DestroyActor`))

(fn `UserConstructionScript`)