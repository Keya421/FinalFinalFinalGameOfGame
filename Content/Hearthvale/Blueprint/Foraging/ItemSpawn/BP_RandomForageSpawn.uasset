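; BP_RandomForageSpawn is a spawn point that periodically produces random forage item pickups at its own transform.
; A looping timer started on BeginPlay rolls against SpawnChance, but only while no previously spawned pickup is still valid; failed rolls print a debug string.
; A successful roll spawns a BP_ItemPickup, assigns a random ItemList entry with a small random stack count, and stores it as Spawned.
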(event `self.ReceiveBeginPlay`
  (`KismetSystemLibrary.K2_SetTimerDelegate` (delegate `RandomSpawn`) (`self.SpawnTime`) true))

(event `RandomSpawn`
  (`/Engine/EditorBlueprintResources/StandardMacros.IsValid` (`self.Spawned`)
    (:`Is Not Valid`
      (if (< (`KismetMathLibrary.RandomFloatInRange` 0.0 100.0) (`self.SpawnChance`))
        (`self.SpawnRandomMaterial`)
        (else
          (`KismetSystemLibrary.PrintString` "fuck"))))))

(fn `SpawnRandomMaterial`
  (bind _returnvalue (`|SpawnActorFromClass` "/Game/Hearthvale/Blueprint/Items/Blueprints/BP_ItemPickup.BP_ItemPickup_C" (`self.GetTransform`) "Undefined" "MultiplyWithRoot" null null))
  (bind _output_get (set `self.Spawned` _returnvalue))
  (set `/Game/Hearthvale/Blueprint/Items/Blueprints/BP_ItemPickup.Item` (`KismetArrayLibrary.Array_Random` (`self.ItemList`)) _output_get)
  (set `/Game/Hearthvale/Blueprint/Items/Blueprints/BP_ItemPickup.ItemCount` (+ (`KismetMathLibrary.RandomInteger` 3) 1) _output_get))

(fn `UserConstructionScript`)