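; Parent tree Blueprint for foraging, providing a function that drops a wood pickup when given a hit location.
; DropWood takes the horizontal direction from the tree toward the hit and spawns a BP_ItemPickup a fixed distance out, with the hit's Z added to the tree's own Z.
; It sets the pickup to a single WoodItem; the event graph and construction script are empty, so DropWood relies on external or child callers.
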(fn `DropWood`
  (params (`Hit Location` :type "Vector Structure"))
  (bind (_returnvalue_x _returnvalue_y) (`KismetMathLibrary.BreakVector` (`self.K2_GetActorLocation`)))
  (bind (_returnvalue_x_2 _returnvalue_y_2) (`KismetMathLibrary.BreakVector` (`KismetMathLibrary.Normal` (- (`KismetMathLibrary.MakeVector` `Hit Location_X` `Hit Location_Y`) (`KismetMathLibrary.MakeVector` _returnvalue_x _returnvalue_y)))))
  (bind _returnvalue (`|SpawnActorFromClass` "/Game/Hearthvale/Blueprint/Items/Blueprints/BP_ItemPickup.BP_ItemPickup_C" (`KismetMathLibrary.MakeTransform` (+ (`KismetMathLibrary.MakeVector` (.x (* (`KismetMathLibrary.MakeVector` _returnvalue_x_2 _returnvalue_y_2) 150.0)) (.y (* (`KismetMathLibrary.MakeVector` _returnvalue_x_2 _returnvalue_y_2) 150.0)) `Hit Location_Z`) (`self.K2_GetActorLocation`))) "Undefined" "MultiplyWithRoot" null null))
  (set `/Game/Hearthvale/Blueprint/Items/Blueprints/BP_ItemPickup.Item` (`self.WoodItem`) _returnvalue)
  (set `/Game/Hearthvale/Blueprint/Items/Blueprints/BP_ItemPickup.ItemCount` 1 _returnvalue))

(fn `UserConstructionScript`)