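; Weather and time-of-day actor that spawns rain, switches cloud cover and sets day or night lighting.
; Rain is an added Niagara component, while clearing destroys it and restores a light-cloud light function on the sun.
; Day and night events retune sun, height fog, sky atmosphere and skylight.
; An optional Tick cycle rotates the sun, flipping it and toggling its color and intensity near the horizon.
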(event `SpawnRain`
  (bind _returnvalue (`AddComponent|NODE_AddNiagaraComponent-0`))
  (bind _output_get (set `self.WeatherComponent` _returnvalue))
  (`NiagaraComponent.SetAsset` _output_get "/Game/Hearthvale/Blueprint/Weather/Niagara/NG_Rain.NG_Rain" true))

(event `ClearWeather`
  (bind _weathercomponent (`self.WeatherComponent`))
  (`/Engine/EditorBlueprintResources/StandardMacros.IsValid` _weathercomponent
    (:`Is Valid`
      (`ActorComponent.K2_DestroyComponent` _weathercomponent))
    (:`Is Not Valid`
      _))
  (`LightComponent.SetLightFunctionMaterial` (`self.SunLight`) "/Game/Hearthvale/Blueprint/Weather/MAT_LightClouds.MAT_LightClouds"))

(event `MakeCloudy`
  (`LightComponent.SetLightFunctionMaterial` (`self.SunLight`) "/Game/Hearthvale/Blueprint/Weather/MAT_HeavyClouds.MAT_HeavyClouds"))

(event `MakeNight`
  (`LightComponent.SetIntensity` (`self.SunLight`) 1.0)
  (`LightComponent.SetLightColor` (`self.SunLight`) (struct :`R` 0.304987 :`G` 0.637597 :`B` 1.0 :`A` 1.0) true)
  (`LightComponent.SetLightColor` (`self.SunLight`) (struct :`R` 0.304987 :`G` 0.637597 :`B` 1.0 :`A` 1.0) true)
  (bind _returnvalue (`GameplayStatics.GetActorOfClass` "/Script/Engine.ExponentialHeightFog"))
  (`ExponentialHeightFogComponent.SetSkyAtmosphereAmbientContributionColorScale` (`ExponentialHeightFog.Component` _returnvalue) (struct :`R` 0.324414 :`G` 0.551799 :`B` 1.0 :`A` 1.0))
  (bind _component (`ExponentialHeightFog.Component` _returnvalue))
  (`ExponentialHeightFogComponent.SetFogHeightFalloff` _component 0.1)
  (`ExponentialHeightFogComponent.SetFogMaxOpacity` (`ExponentialHeightFog.Component` _returnvalue) 1.0)
  (`ExponentialHeightFogComponent.SetVolumetricFog` _component false)
  (`ExponentialHeightFogComponent.SetVolumetricFogScatteringDistribution` _component 0.1)
  (`ExponentialHeightFogComponent.SetVolumetricFogExtinctionScale` _component 0.5)
  (bind _returnvalue_2 (`GameplayStatics.GetActorOfClass` "/Script/Engine.SkyAtmosphere"))
  (`SkyAtmosphereComponent.SetAtmosphereHeight` (`SkyAtmosphere.SkyAtmosphereComponent` _returnvalue_2) 5.0)
  (bind _returnvalue_3 (`GameplayStatics.GetActorOfClass` "/Script/Engine.SkyLight"))
  (bind _lightcomponent (`SkyLight.LightComponent` _returnvalue_3))
  (`SkyLightComponent.SetIntensity` _lightcomponent 2.0)
  (`SkyLightComponent.SetLightColor` _lightcomponent (struct :`R` 0.630208 :`G` 0.807178 :`B` 1.0 :`A` 1.0))
  (`GameplayStatics.GetActorOfClass` "/Script/Engine.PostProcessVolume"))

(event `self.ReceiveTick`
  (params (DeltaSeconds :type "Float (single-precision)"))
  (bind _sunlight (`self.SunLight`))
  (bind (_returnvalue_roll _returnvalue_pitch) (`KismetMathLibrary.BreakRotator` (`SceneComponent.K2_GetComponentRotation` (`self.SunLight`))))
  (if (`self.Day/Night Cycle?`)
    (`SceneComponent.K2_AddLocalRotation` (`self.SunLight`) (`KismetMathLibrary.MakeRotator` 0.0 (* DeltaSeconds (`self.DayLength`))) false false)
    (if (`KismetMathLibrary.NearlyEqual_FloatFloat` (`KismetMathLibrary.Abs` _returnvalue_pitch) 0.0 10.0)
      (`/Engine/EditorBlueprintResources/StandardMacros.DoOnce` false :!label _label
        (:`Completed`
          (if (`self.night`)
            (set `self.night` false)
            (`LightComponent.SetLightColor` _sunlight (struct :`R` 1.0 :`G` 1.0 :`B` 1.0 :`A` 1.0) true)
            (`LightComponent.SetIntensity` _sunlight 2.5)
            (else
              (set `self.night` true)
              (`KismetSystemLibrary.PrintString` "Hello")
              (`LightComponent.SetLightColor` _sunlight (struct :`R` 0.443399 :`G` 0.659116 :`B` 1.0 :`A` 1.0) true)
              (`LightComponent.SetIntensity` _sunlight 1.0)))
          (`SceneComponent.K2_AddLocalRotation` (`self.SunLight`) (struct :`Pitch` -10.0 :`Yaw` 180.0 :`Roll` 180.0) false false)
          (`KismetSystemLibrary.Delay` 1.0)
          (goto _label :!via `Reset`))))))

(event `Make Daytime`
  (`LightComponent.SetIntensity` (`self.SunLight`) 2.5)
  (`LightComponent.SetLightColor` (`self.SunLight`) (struct :`R` 1.0 :`G` 1.0 :`B` 1.0 :`A` 1.0) true)
  (`LightComponent.SetLightColor` (`self.SunLight`) (struct :`R` 1.0 :`G` 1.0 :`B` 1.0 :`A` 1.0) true)
  (bind _returnvalue (`GameplayStatics.GetActorOfClass` "/Script/Engine.ExponentialHeightFog"))
  (`ExponentialHeightFogComponent.SetSkyAtmosphereAmbientContributionColorScale` (`ExponentialHeightFog.Component` _returnvalue) (struct :`R` 1.0 :`G` 1.0 :`B` 1.0 :`A` 1.0))
  (bind _component (`ExponentialHeightFog.Component` _returnvalue))
  (`ExponentialHeightFogComponent.SetFogHeightFalloff` _component 0.1)
  (`ExponentialHeightFogComponent.SetFogMaxOpacity` (`ExponentialHeightFog.Component` _returnvalue) 1.0)
  (`ExponentialHeightFogComponent.SetVolumetricFog` _component true)
  (`ExponentialHeightFogComponent.SetVolumetricFogScatteringDistribution` _component 0.1)
  (`ExponentialHeightFogComponent.SetVolumetricFogExtinctionScale` _component 0.5)
  (bind _returnvalue_2 (`GameplayStatics.GetActorOfClass` "/Script/Engine.SkyAtmosphere"))
  (`SkyAtmosphereComponent.SetAtmosphereHeight` (`SkyAtmosphere.SkyAtmosphereComponent` _returnvalue_2) 5.0)
  (bind _returnvalue_3 (`GameplayStatics.GetActorOfClass` "/Script/Engine.SkyLight"))
  (bind _lightcomponent (`SkyLight.LightComponent` _returnvalue_3))
  (`SkyLightComponent.SetIntensity` _lightcomponent 2.0)
  (`SkyLightComponent.SetLightColor` _lightcomponent (struct :`R` 1.0 :`G` 1.0 :`B` 1.0 :`A` 1.0))
  (`GameplayStatics.GetActorOfClass` "/Script/Engine.PostProcessVolume"))

(fn `UserConstructionScript`)