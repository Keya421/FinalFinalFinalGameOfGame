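; House is a restaurant entrance trigger that gates travel to the restaurant level behind the player's gathering progress.
; When the third-person character overlaps the box, it checks that character's wood, crop and fish flags in that order.
; With all three met it opens the restaurant level; otherwise it starts a dialogue on the character naming the first missing task.
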(event `self.Box.OnComponentBeginOverlap`
  (params (OverlappedComponent :type "PrimitiveComponent Object Reference") (OtherActor :type "Actor Object Reference") (OtherComp :type "PrimitiveComponent Object Reference") (OtherBodyIndex :type Integer) (bFromSweep :type Boolean) (SweepResult :type "HitResult Structure (by ref)"))
  (bind _asbp_third_person_character (cast `/Game/ThirdPerson/Blueprints/BP_ThirdPersonCharacter` OtherActor))
  (if (`/Game/ThirdPerson/Blueprints/BP_ThirdPersonCharacter.5Wood?` _asbp_third_person_character)
    (if (`/Game/ThirdPerson/Blueprints/BP_ThirdPersonCharacter.Crop?` _asbp_third_person_character)
      (if (`/Game/ThirdPerson/Blueprints/BP_ThirdPersonCharacter.fish?` _asbp_third_person_character)
        (`GameplayStatics.OpenLevelBySoftObjectPtr` "/Game/Hearthvale/GameMap/RestaurantLevel.RestaurantLevel")
        (else
          (`/Game/ThirdPerson/Blueprints/BP_ThirdPersonCharacter.StartDialogue` _asbp_third_person_character (`|MakeArray` (make `/Game/Hearthvale/Blueprint/UI/Dialogue/ST_DialogueOptions` "You still need to catch a fish before you go there! " 1 null _ true) :!type "/Game/Hearthvale/Blueprint/UI/Dialogue/ST_DialogueOptions Structure"))))
      (else
        (`/Game/ThirdPerson/Blueprints/BP_ThirdPersonCharacter.StartDialogue` _asbp_third_person_character (`|MakeArray` (make `/Game/Hearthvale/Blueprint/UI/Dialogue/ST_DialogueOptions` "You still need to harvest some crops before you go there!" 1 null _ true) :!type "/Game/Hearthvale/Blueprint/UI/Dialogue/ST_DialogueOptions Structure"))))
    (else
      (`/Game/ThirdPerson/Blueprints/BP_ThirdPersonCharacter.StartDialogue` _asbp_third_person_character (`|MakeArray` (make `/Game/Hearthvale/Blueprint/UI/Dialogue/ST_DialogueOptions` "You still need to chop down 5 trees before you go there!" 1 null _ true) :!type "/Game/Hearthvale/Blueprint/UI/Dialogue/ST_DialogueOptions Structure")))))

(fn `UserConstructionScript`)