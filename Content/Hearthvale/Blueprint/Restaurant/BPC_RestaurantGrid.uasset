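; BPC_RestaurantGrid is a component that provides grid placement helpers for the restaurant.
; GetGridLocation snaps X and Y to the nearest cell center using GridSize and keeps Z.
; OverlapCheck runs a zero-length box trace on Visibility, skipping ignored actors, and returns whether a Length by Width footprint is blocked.
; The box is slightly inset, assumes 100-unit cells regardless of GridSize, and draws timed debug shapes.
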(fn `Get Grid Location`
  (params (Location :type "Vector Structure"))
  (returns (GridLocation :type "Vector Structure"))
  (bind _gridsize (`self.GridSize`))
  (bind _gridsize_2 (`self.GridSize`))
  (bind _returnvalue (/ (`self.GridSize`) 2.0))
  (bind _returnvalue_2 (/ _gridsize_2 2.0))
  (return (`KismetMathLibrary.MakeVector` (+ (* (`KismetMathLibrary.Conv_IntToDouble` (`KismetMathLibrary.Round` (/ (- Location_X _returnvalue) _gridsize))) _gridsize_2) _returnvalue_2) (+ (* (`KismetMathLibrary.Conv_IntToDouble` (`KismetMathLibrary.Round` (/ (- Location_Y _returnvalue) _gridsize))) _gridsize_2) _returnvalue_2) Location_Z)))

(fn `OverlapCheck`
  (params (SpawnLocation :type "Vector Structure") (Length :type Integer) (Width :type Integer) (IgnoreActors :type "Array of Actor Object Reference"))
  (returns (`Overlap?` :type Boolean))
  (bind _outhit (`KismetSystemLibrary.BoxTraceSingle` SpawnLocation SpawnLocation (`KismetMathLibrary.MakeVector` (* Length 49.9) (* Width 49.9) 50.0) (struct) "TraceTypeQuery1" false IgnoreActors "ForDuration"))
  (return (`GameplayStatics.BreakHitResult` _outhit)))