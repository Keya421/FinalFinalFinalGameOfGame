(event `/Game/Hearthvale/Blueprint/PlayerData/BPI_Interact.Interact`
  (params (`Hit Component` :type "ActorComponent Object Reference"))
  (`/Game/ThirdPerson/Blueprints/BP_ThirdPersonCharacter.StartDialogue` (cast `/Game/ThirdPerson/Blueprints/BP_ThirdPersonCharacter` (`GameplayStatics.GetPlayerPawn` 0) :!pure true) (`|MakeArray` (make `/Game/Hearthvale/Blueprint/UI/Dialogue/ST_DialogueOptions` "What would you like to do?" 0 null (`|MakeArray` (make `/Game/Hearthvale/Blueprint/UI/Dialogue/ST_DialogueOpenEnded` "Save and Quit" 0 0 true true) (make `/Game/Hearthvale/Blueprint/UI/Dialogue/ST_DialogueOpenEnded` "Save" 0 1 true true) (make `/Game/Hearthvale/Blueprint/UI/Dialogue/ST_DialogueOpenEnded` "Cancel" 0 99 false true) :!type "/Game/Hearthvale/Blueprint/UI/Dialogue/ST_DialogueOpenEnded Structure")) :!type "/Game/Hearthvale/Blueprint/UI/Dialogue/ST_DialogueOptions Structure"))
  (add `/Game/Hearthvale/A/UI-AP/DialogueTest.ReturnIndex` (`/Game/ThirdPerson/Blueprints/BP_ThirdPersonCharacter.DialogueWidget` (cast `/Game/ThirdPerson/Blueprints/BP_ThirdPersonCharacter` (`GameplayStatics.GetPlayerPawn` 0) :!pure true)) (delegate `OnSelected`)))

(event `OnSelected`
  (params (Index :type Integer))
  (bind _asgi_hearthvale (cast `/Game/Hearthvale/Blueprint/GI_Hearthvale` (`GameplayStatics.GetGameInstance`) :!pure true))
  (switch `int` Index
    (:`0`
      (`/Game/Hearthvale/Blueprint/GI_Hearthvale.SaveGame` _asgi_hearthvale "1" true))
    (:`1`
      (`/Game/Hearthvale/Blueprint/GI_Hearthvale.SaveGame` _asgi_hearthvale "1" false))))

(event `/Game/Hearthvale/Blueprint/PlayerData/BPI_Interact.ShowInteract`
  (`/Game/ThirdPerson/Blueprints/BP_ThirdPersonCharacter.SetInteractWidget` (cast `/Game/ThirdPerson/Blueprints/BP_ThirdPersonCharacter` (`GameplayStatics.GetPlayerPawn` 0) :!pure true) (`|MakeArray` (make `/Game/Hearthvale/Blueprint/UI/Interact/ST_InteractSettings` "Your bed" "" false 0 null) :!type "/Game/Hearthvale/Blueprint/UI/Interact/ST_InteractSettings Structure") self))

(fn `UserConstructionScript`)