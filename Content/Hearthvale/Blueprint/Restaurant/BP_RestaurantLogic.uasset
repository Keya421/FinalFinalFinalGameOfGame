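; Restaurant logic Blueprint that spawns customers, seats them, builds their orders and places furniture.
; SpawnCustomer sizes each party up to the largest free table and gives it random dishes, loaded through the Asset Registry from the Dishes folder.
; AcceptCustomer assigns party and order to the smallest free table that fits, found by pruning a table-to-chair-count map.
; PlaceFurniture uses a temporary checker actor to test grid overlap before spawning furniture ahead of the player.
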(fn `AcceptCustomer`
  (params (CustomerAmount :type Integer) (CustomerRef :type "/Game/Hearthvale/Blueprint/Restaurant/Actors/Customer/BP_Customer Object Reference") (CustomerOrder :type "Array of /Game/Hearthvale/Blueprint/Items/ItemData/Food/DA_ItemFood Class Reference"))
  (bind _availabletable (`self.FindAvailableTable` CustomerAmount))
  (set `/Game/Hearthvale/Blueprint/Restaurant/Actors/Furniture/Seating/zParentClasses/BP_TableParent.AssignedCustomer` CustomerRef _availabletable)
  (set `/Game/Hearthvale/Blueprint/Restaurant/Actors/Furniture/Seating/zParentClasses/BP_TableParent.AssignedOrder` CustomerOrder _availabletable)
  (`/Game/Hearthvale/Blueprint/Restaurant/Actors/Customer/BP_Customer.GoToTable` CustomerRef _availabletable))

(fn `CreateOrder`
  (params (NumberOfCustomers :type Integer))
  (returns (Order :type "Array of /Game/Hearthvale/Blueprint/Items/ItemData/Food/DA_ItemFood Class Reference"))
  (locals (Order :type "Array of /Game/Hearthvale/Blueprint/Items/ItemData/Food/DA_ItemFood Class Reference") (DishList :type "Array of /Game/Hearthvale/Blueprint/Items/ItemData/Food/DA_ItemFood Class Reference") (TimesAdded :type Integer))
  (bind _alldishclasses (`self.GetAllDishes`))
  (set `local.DishList` _alldishclasses)
  (while (>= NumberOfCustomers (+ (`KismetArrayLibrary.Array_Length` (`local.Order`)) 1))
    (`KismetArrayLibrary.Array_Add` (`local.Order`) (`KismetArrayLibrary.Array_Random` (`local.DishList`))))
  (return (`local.Order`)))

(fn `FindAvailableTable`
  (params (NumCustomers :type Integer))
  (returns (AvailableTable :type "/Game/Hearthvale/Blueprint/Restaurant/Actors/Furniture/Seating/zParentClasses/BP_TableParent Object Reference"))
  (locals (TableList :type "Map of /Game/Hearthvale/Blueprint/Restaurant/Actors/Furniture/Seating/zParentClasses/BP_TableParent Object Reference to Object Object Reference") (TableSizeInt :type "Map of Integer to Object Object Reference") (NumberOfCustomers :type Integer) (Unfinished :type Boolean :default true) (SelectedTable :type "/Game/Hearthvale/Blueprint/Restaurant/Actors/Furniture/Seating/zParentClasses/BP_TableParent Object Reference") (Failed :type Boolean))
  (bind _selectedtable (`local.SelectedTable`))
  (bind _tablelist (`local.TableList`))
  (set `local.NumberOfCustomers` NumCustomers)
  (bind _tablelist_2 (`self.GetTableList`))
  (set `local.TableList` _tablelist_2)
  (while (`local.Unfinished`)
    (bind _values (`BlueprintMapLibrary.Map_Values` (`local.TableList`)))
    (if (`BlueprintMapLibrary.Map_IsEmpty` _tablelist)
      (`KismetSystemLibrary.PrintString` "No Available Seat fuckass")
      (set `local.Unfinished` false)
      (set `local.Failed` true)
      (else
        (bind _key (`BlueprintMapLibrary.Map_GetKeyValueByIndex` _tablelist (`KismetMathLibrary.MinOfIntArray` _values)))
        (if (`/Game/Hearthvale/Blueprint/Restaurant/Actors/Furniture/Seating/zParentClasses/BP_TableParent.isTableNotTaken` _key)
          (if (>= (`/Game/Hearthvale/Blueprint/Restaurant/Actors/Furniture/Seating/zParentClasses/BP_TableParent.SurroundingChairs` _key) (`local.NumberOfCustomers`))
            (set `local.Unfinished` false)
            (set `local.SelectedTable` _key)
            (else
              (`BlueprintMapLibrary.Map_Remove` (`local.TableList`) _key :!label _label)))
          (else
            (goto _label))))))
  (if (`local.Failed`)
    (`KismetSystemLibrary.PrintString` "its so joever")
    (else
      (`KismetSystemLibrary.PrintString` "HOLY TABLE WIN")
      (`KismetSystemLibrary.PrintString` (`KismetSystemLibrary.GetDisplayName` _selectedtable))
      (return _selectedtable))))

(fn `FindHighestAvailableSeatCount`
  (returns (HighestSeatCount :type Integer))
  (locals (TempTableList :type "Map of /Game/Hearthvale/Blueprint/Restaurant/Actors/Furniture/Seating/zParentClasses/BP_TableParent Object Reference to Object Object Reference"))
  (bind _tablelist (`self.GetTableList`))
  (bind _output_get (set `local.TempTableList` _tablelist))
  (bind _values (`BlueprintMapLibrary.Map_Values` _output_get :!label _label))
  (if (`KismetArrayLibrary.Array_IsNotEmpty` _values)
    (bind (_indexofmaxvalue _maxvalue) (`KismetMathLibrary.MaxOfIntArray` _values))
    (bind _key (`BlueprintMapLibrary.Map_GetKeyValueByIndex` _output_get _indexofmaxvalue))
    (if (`/Game/Hearthvale/Blueprint/Restaurant/Actors/Furniture/Seating/zParentClasses/BP_TableParent.isTableNotTaken` _key)
      (return _maxvalue)
      (else
        (`BlueprintMapLibrary.Map_Remove` _output_get _key)
        (goto _label)))
    (else
      (return 0))))

(fn `GetAllDishes`
  (returns (AllDishClasses :type "Array of /Game/Hearthvale/Blueprint/Items/ItemData/Food/DA_ItemFood Class Reference"))
  (locals (Dishes :type "Array of /Game/Hearthvale/Blueprint/Items/ItemData/Food/DA_ItemFood Class Reference"))
  (bind _outassetdata (`AssetRegistry.GetAssetsByPath` (`AssetRegistryHelpers.GetAssetRegistry`) "/Game/Hearthvale/Blueprint/Items/ItemData/Food/Dishes" false false))
  (for _array_element _outassetdata
    (bind (_packagename _packagepath _assetname) (break `AssetData` _array_element))
    (bind _returnvalue (`KismetSystemLibrary.LoadClassAsset_Blocking` (`KismetSystemLibrary.Conv_SoftClassPathToSoftClassRef` (`KismetSystemLibrary.MakeSoftClassPath` (`KismetStringLibrary.Concat_StrStr` (`KismetStringLibrary.Conv_NameToString` _packagename) "." (`KismetStringLibrary.Conv_NameToString` _assetname) "_C")))))
    (bind _asda_item_food (castclass `/Game/Hearthvale/Blueprint/Items/ItemData/Food/DA_ItemFood` _returnvalue))
    (`KismetArrayLibrary.Array_AddUnique` (`local.Dishes`) _asda_item_food))
  (return (`local.Dishes`)))

(fn `GetTableList`
  (returns (TableList :type "Map of /Game/Hearthvale/Blueprint/Restaurant/Actors/Furniture/Seating/zParentClasses/BP_TableParent Object Reference to Integer"))
  (locals (TableList :type "Map of /Game/Hearthvale/Blueprint/Restaurant/Actors/Furniture/Seating/zParentClasses/BP_TableParent Object Reference to Object Object Reference"))
  (bind _outactors (`GameplayStatics.GetAllActorsOfClass` "/Game/Hearthvale/Blueprint/Restaurant/Actors/Furniture/Seating/zParentClasses/BP_TableParent.BP_TableParent_C"))
  (for _array_element _outactors
    (`BlueprintMapLibrary.Map_Add` (`local.TableList`) _array_element (`/Game/Hearthvale/Blueprint/Restaurant/Actors/Furniture/Seating/zParentClasses/BP_TableParent.SurroundingChairs` _array_element)))
  (return (`local.TableList`)))

(fn `PlaceFurniture`
  (params (Furniture :type "/Game/Hearthvale/Blueprint/Items/ItemData/Restaurant/DA_ItemFurniture Class Reference"))
  (returns (`Success?` :type Boolean))
  (locals (NoOverlap :type Boolean))
  (bind (_gridwidth _gridlength _furnitureactorref) (defaults `Object` Furniture))
  (bind _asbp_third_person_character (cast `/Game/ThirdPerson/Blueprints/BP_ThirdPersonCharacter` (`Controller.K2_GetPawn` (`GameplayStatics.GetPlayerController` 0)) :!pure true))
  (bind _gridlocation (`/Game/Hearthvale/Blueprint/Restaurant/BPC_RestaurantGrid.Get Grid Location` (`self.BPC_RestaurantGrid`) (+ (* (`self.GetActorForwardVector` _asbp_third_person_character) 50.0) (`self.K2_GetActorLocation` _asbp_third_person_character))))
  (bind _returnvalue (`|SpawnActorFromClass` "/Game/Hearthvale/Blueprint/Restaurant/BP_FurnitureCheck.BP_FurnitureCheck_C" (`KismetMathLibrary.MakeTransform` _gridlocation) "Undefined" "MultiplyWithRoot" null null))
  (set `/Game/Hearthvale/Blueprint/Restaurant/BP_FurnitureCheck.FurnitureWidth` _gridwidth _returnvalue)
  (set `/Game/Hearthvale/Blueprint/Restaurant/BP_FurnitureCheck.FurnitureLength` _gridlength _returnvalue)
  (bind (_nooverlap _rotation) (`/Game/Hearthvale/Blueprint/Restaurant/BP_FurnitureCheck.CheckOverlap` _returnvalue))
  (bind _output_get (set `local.NoOverlap` _nooverlap))
  (if _output_get
    (`self.K2_DestroyActor` _returnvalue)
    (bind _returnvalue_2 (`|SpawnActorFromClass` _furnitureactorref (`KismetMathLibrary.MakeTransform` _gridlocation (`KismetMathLibrary.MakeRotator` 0.0 0.0 (`KismetMathLibrary.Conv_IntToDouble` (* _rotation 90))) (0.0 0.0 0.0)) "Undefined" "MultiplyWithRoot" null null))
    (set `/Game/Hearthvale/Blueprint/Restaurant/Actors/BP_RestaurantDecor.Width` _gridwidth _returnvalue_2)
    (set `/Game/Hearthvale/Blueprint/Restaurant/Actors/BP_RestaurantDecor.Length` _gridlength _returnvalue_2)
    (return true)
    (else
      (`self.K2_DestroyActor` _returnvalue)
      (`KismetSystemLibrary.PrintString` "Give Fail to place message to player")
      (return false))))

(fn `SpawnCustomer`
  (bind _highestseatcount (`self.FindHighestAvailableSeatCount`))
  (if (<= _highestseatcount 0)
    (`KismetSystemLibrary.PrintString` "NoAvailableSeats, will not spawn.")
    (else
      (bind _outactors (`GameplayStatics.GetAllActorsOfClass` "/Game/Hearthvale/Blueprint/Restaurant/Actors/Customer/BP_CustomerSpawn.BP_CustomerSpawn_C"))
      (bind _returnvalue (`|SpawnActorFromClass` "/Game/Hearthvale/Blueprint/Restaurant/Actors/Customer/BP_Customer.BP_Customer_C" (`self.GetTransform` (`|GetArrayItem` _outactors)) "Undefined" "MultiplyWithRoot" null null))
      (bind _output_get (set `/Game/Hearthvale/Blueprint/Restaurant/Actors/Customer/BP_Customer.CustomerCount` (`KismetMathLibrary.RandomIntegerInRange` 1 _highestseatcount) _returnvalue))
      (bind _order (`self.CreateOrder` _output_get))
      (set `/Game/Hearthvale/Blueprint/Restaurant/Actors/Customer/BP_Customer.CustomerOrder` _order _returnvalue))))

(fn `UserConstructionScript`)