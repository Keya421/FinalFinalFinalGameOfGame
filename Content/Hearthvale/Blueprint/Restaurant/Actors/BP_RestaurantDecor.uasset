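; Restaurant decor actor that aligns itself to the restaurant grid and rests on the surface beneath it.
; The construction script snaps its location through BPCRestaurantGrid unless MoveActor is set.
; BeginPlay snaps again, then runs a short Visibility trace along the actor's down vector and moves it to the hit point.
; If nothing is hit, it stays at the grid location and prints debug messages.
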(event `self.ReceiveBeginPlay`
  (bind _returnvalue (`self.K2_GetActorLocation`))
  (bind _gridlocation (`/Game/Hearthvale/Blueprint/Restaurant/BPC_RestaurantGrid.Get Grid Location` (`self.BPC_RestaurantGrid`) (`self.K2_GetActorLocation`)))
  (`self.K2_SetActorLocation` _gridlocation)
  (bind _outhit (`KismetSystemLibrary.LineTraceSingle` _returnvalue (+ (* (* (`self.GetActorUpVector`) -1.0) 500.0) _returnvalue) "TraceTypeQuery1"))
  (bind (_bblockinghit _binitialoverlap _time _distance _location) (`GameplayStatics.BreakHitResult` _outhit))
  (if _bblockinghit
    (`self.K2_SetActorLocation` _location)
    (else
      (`KismetSystemLibrary.PrintString` "where the fuck are you?")
      (`KismetSystemLibrary.PrintString` "you're probably in the air, so i couldnt place it down to the ground."))))

(fn `UserConstructionScript`
  (if (not (`self.MoveActor`))
    (bind _gridlocation (`/Game/Hearthvale/Blueprint/Restaurant/BPC_RestaurantGrid.Get Grid Location` (`self.BPC_RestaurantGrid`) (`self.K2_GetActorLocation`)))
    (`self.K2_SetActorLocation` _gridlocation)))