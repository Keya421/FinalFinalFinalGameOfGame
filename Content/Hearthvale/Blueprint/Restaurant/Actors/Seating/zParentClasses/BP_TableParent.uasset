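; Parent Blueprint for restaurant tables that keeps a count of the chairs around it.
; The construction script scales the actor by table length and width, then runs the chair count.
; FindSurroundingChairs stores the number of overlapping BP_ChairParent actors, or zero if there are none.
; The count refreshes on BeginPlay and whenever any actor begins or ends overlapping the table.
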(event `self.ReceiveBeginPlay`
  (`parent.ReceiveBeginPlay`)
  (`self.FindSurroundingChairs` :!label _label))

(event `self.ReceiveActorBeginOverlap`
  (params (OtherActor :type "Actor Object Reference"))
  (`parent.ReceiveActorBeginOverlap` OtherActor)
  (goto _label))

(event `self.ReceiveActorEndOverlap`
  (params (OtherActor :type "Actor Object Reference"))
  (goto _label))

(fn `FindSurroundingChairs`
  (bind _overlappingactors (`self.GetOverlappingActors` "/Game/Hearthvale/Blueprint/Restaurant/Actors/Seating/zParentClasses/BP_ChairParent.BP_ChairParent_C"))
  (if (`KismetArrayLibrary.Array_IsValidIndex` _overlappingactors)
    (set `self.SurroundingChairs` (`KismetArrayLibrary.Array_Length` _overlappingactors))
    (else
      (set `self.SurroundingChairs` 0))))

(fn `UserConstructionScript`
  (`parent.UserConstructionScript`)
  (`self.SetActorScale3D` (`KismetMathLibrary.MakeVector` (`KismetMathLibrary.Conv_IntToDouble` (`self.TableLength`)) (`KismetMathLibrary.Conv_IntToDouble` (`self.TableWidth`)) 1.0))
  (`self.FindSurroundingChairs`))