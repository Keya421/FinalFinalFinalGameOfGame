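; BP_StorageChest is a furniture actor for the restaurant that acts as an interactable storage chest.
; ShowInteract sends a "Storage Chest" prompt, along with its child interact entries, to the player character's interact widget.
; Interact creates the WB_chestInventory widget, passes it the chest and its ChestStorage contents, then switches to UI-only input with a visible mouse.
; Construction only calls the parent script.
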(event `/Game/Hearthvale/Blueprint/PlayerData/BPI_Interact.Interact`
  (params (`Hit Component` :type "ActorComponent Object Reference"))
  (bind _returnvalue (`|CreateWidget` "/Game/Hearthvale/Blueprint/storage/WB_chestInventory.WB_chestInventory_C" (`GameplayStatics.GetPlayerController` 0)))
  (set `/Game/Hearthvale/Blueprint/storage/WB_chestInventory.storge` (`|ConvertAsset` self) _returnvalue)
  (set `/Game/Hearthvale/Blueprint/storage/WB_chestInventory.SavedStorage` (`self.chestStorage`) _returnvalue)
  (`UserWidget.AddToViewport` _returnvalue 0)
  (`WidgetBlueprintLibrary.SetInputMode_UIOnlyEx` (`GameplayStatics.GetPlayerController` 0) null)
  (`/Game/ThirdPerson/Blueprints/BP_ThirdPersonCharacter.EnableShowMouse` (cast `/Game/ThirdPerson/Blueprints/BP_ThirdPersonCharacter` (`GameplayStatics.GetPlayerPawn` 0) :!pure true) true))

(event `/Game/Hearthvale/Blueprint/PlayerData/BPI_Interact.ShowInteract`
  (`/Game/ThirdPerson/Blueprints/BP_ThirdPersonCharacter.SetInteractWidget` (cast `/Game/ThirdPerson/Blueprints/BP_ThirdPersonCharacter` (`GameplayStatics.GetPlayerPawn` 0) :!pure true) (`|MakeArray` (make `/Game/Hearthvale/Blueprint/UI/Interact/ST_InteractSettings` "Storage Chest") (`self.ChildInteract`) (`self.ChildInteract2`)) self))

(fn `UserConstructionScript`
  (`parent.UserConstructionScript`))