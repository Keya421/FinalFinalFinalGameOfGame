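; A restaurant customer party actor that asks for a table through dialogue, with a vendor variant that skips dialogue and random textures.
; It shows the component group matching party size, capped at four, using dynamic materials with random textures loaded from a folder via Asset Registry.
; Accepting the dialogue passes party and order to BP_RestaurantLogic.
; GoToTable hands the textures to the table's seats and destroys the actor.
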(event `self.ReceiveBeginPlay`
  (`KismetSystemLibrary.Delay` 0.0001)
  (if (`self.bIsVendor?`)
    (`self.UpdateVisibleCustomers`)
    (`PrimitiveComponent.SetMaterial` (`self.Cylinder`) 0 "/Engine/MaterialTemplates/VertexAnimation/AdvancedFlag.AdvancedFlag")
    (else
      (`self.UpdateVisibleCustomers`)
      (`self.GetRandomTextures`)
      (`self.AssignRandomCustomerTextures`))))

(event `/Game/Hearthvale/Blueprint/PlayerData/BPI_Interact.Interact`
  (bind _asbp_third_person_character (cast `/Game/ThirdPerson/Blueprints/BP_ThirdPersonCharacter` (`Controller.K2_GetPawn` (`GameplayStatics.GetPlayerController` 0)) :!pure true))
  (if (not (`self.bIsVendor?`))
    (set `self.Dialogue` (`|MakeArray` (make `/Game/Hearthvale/Blueprint/UI/Dialogue/ST_DialogueOptions` (`KismetTextLibrary.Conv_StringToText` (`KismetStringLibrary.Concat_StrStr` "Table for " (`KismetStringLibrary.Conv_IntToString` (`self.CustomerCount`)) ", please!")) 0 "/Game/Hearthvale/A/UI-AP/Emu_03_prsk_erica_moe.Emu_03_prsk_erica_moe" (`|MakeArray` (make `/Game/Hearthvale/Blueprint/UI/Dialogue/ST_DialogueOpenEnded` "Alright!" 0 0 true true) (make `/Game/Hearthvale/Blueprint/UI/Dialogue/ST_DialogueOpenEnded` "fuck you" 0 1 true true) :!type "/Game/Hearthvale/Blueprint/UI/Dialogue/ST_DialogueOpenEnded Structure") true) :!type "/Game/Hearthvale/Blueprint/UI/Dialogue/ST_DialogueOptions Structure"))
    (`/Game/ThirdPerson/Blueprints/BP_ThirdPersonCharacter.StartDialogue` _asbp_third_person_character (`self.Dialogue`))
    (add `/Game/Hearthvale/A/UI-AP/DialogueTest.ReturnIndex` (`/Game/ThirdPerson/Blueprints/BP_ThirdPersonCharacter.DialogueWidget` _asbp_third_person_character) (delegate `OnSelected`))))

(event `OnSelected`
  (params (Index :type Integer))
  (switch `int` Index
    (:`0`
      (bind _returnvalue (`GameplayStatics.GetActorOfClass` "/Game/Hearthvale/Blueprint/Restaurant/BP_RestaurantLogic.BP_RestaurantLogic_C"))
      (`/Game/Hearthvale/Blueprint/Restaurant/BP_RestaurantLogic.AcceptCustomer` _returnvalue (`self.CustomerCount`) self (`self.CustomerOrder`)))))

(fn `AcceptCustomerOrder`
  (bind _returnvalue (`GameplayStatics.GetActorOfClass` "/Game/Hearthvale/Blueprint/Restaurant/BP_RestaurantLogic.BP_RestaurantLogic_C"))
  (`/Game/Hearthvale/Blueprint/Restaurant/BP_RestaurantLogic.AcceptCustomer` _returnvalue (`self.CustomerCount`) self (`self.CustomerOrder`)))

(fn `AssignRandomCustomerTextures`
  (locals (SceneComponent :type "SceneComponent Object Reference") (Added :type Integer) (Selected :type "PrimitiveComponent Object Reference"))
  (switch `int` (- (`self.CustomerCount`) 1)
    (:`0`
      (set `local.SceneComponent` (`self.1OneCustomer`)))
    (:`1`
      (set `local.SceneComponent` (`self.2TwoCustomer`)))
    (:`2`
      (set `local.SceneComponent` (`self.3ThreeCustomer`)))
    (:`3`
      (set `local.SceneComponent` (`self.4FourCustomer`))))
  (for (_array_element _array_index) (`SceneComponent.GetChildrenComponents` (`local.SceneComponent`) false)
    (bind _asprimitive_component (cast `PrimitiveComponent` _array_element))
    (bind _returnvalue (`PrimitiveComponent.CreateDynamicMaterialInstance` _asprimitive_component 0 "/Game/Hearthvale/Materials/CustomerMaterials/MAT_Customer.MAT_Customer" "None"))
    (`MaterialInstanceDynamic.SetTextureParameterValue` _returnvalue "CustomerTexture" (`|GetArrayItem` (`self.CustomerTextures`) _array_index))))

(fn `GetRandomTextures`
  (locals (AllTexturesArray :type "Array of Texture2D Object Reference"))
  (bind _outassetdata (`AssetRegistry.GetAssetsByPath` (`AssetRegistryHelpers.GetAssetRegistry`) "/Game/Hearthvale/Textures/CustomerTextures" false false))
  (for _array_element _outassetdata
    (bind _astexture_2d (cast `Texture2D` (`AssetRegistryHelpers.GetAsset` _array_element))
      (:`then`
        (`KismetArrayLibrary.Array_AddUnique` (`local.AllTexturesArray`) _astexture_2d))
      (:`CastFailed`
        (`KismetSystemLibrary.PrintString` "fail"))))
  (while (> (`self.CustomerCount`) (`KismetArrayLibrary.Array_Length` (`self.CustomerTextures`)))
    (`KismetArrayLibrary.Array_Add` (`self.CustomerTextures`) (`KismetArrayLibrary.Array_Random` (`local.AllTexturesArray`)))))

(fn `GoToTable`
  (params (TableRef :type "/Game/Hearthvale/Blueprint/Restaurant/Actors/Furniture/Seating/zParentClasses/BP_TableParent Object Reference"))
  (`/Game/Hearthvale/Blueprint/Restaurant/Actors/Furniture/Seating/zParentClasses/BP_TableParent.AssignCustomersToSeats` TableRef (`self.CustomerTextures`))
  (`self.K2_DestroyActor`))

(fn `UpdateVisibleCustomers`
  (locals (VisibleCustomer :type Integer :default 1) (VisibleComp :type "SceneComponent Object Reference"))
  (bind _customercount (`self.CustomerCount`))
  (for _array_element (`|MakeArray` (`self.1OneCustomer`) (`self.2TwoCustomer`) (`self.3ThreeCustomer`) (`self.4FourCustomer`))
    (for _array_element_2 (`SceneComponent.GetChildrenComponents` _array_element false)
      (`SceneComponent.SetVisibility` _array_element_2 false true)))
  (if (> _customercount 4)
    (set `local.VisibleCustomer` 4)
    (else
      (set `local.VisibleCustomer` _customercount)))
  (switch `int` (`local.VisibleCustomer`)
    (:`Default`
      (`KismetSystemLibrary.RaiseScriptError` "CustomerCount is invalid. What the hell?" :!label _label))
    (:`0`
      (goto _label))
    (:`1`
      (set `local.VisibleComp` (`self.1OneCustomer`))
      (`SceneComponent.SetVisibility` (`local.VisibleComp`) true true :!label _label_2))
    (:`2`
      (set `local.VisibleComp` (`self.2TwoCustomer`))
      (goto _label_2))
    (:`3`
      (set `local.VisibleComp` (`self.3ThreeCustomer`))
      (goto _label_2))
    (:`4`
      (set `local.VisibleComp` (`self.4FourCustomer`))
      (goto _label_2))))

(fn `UserConstructionScript`
  (locals (VisibileComp :type "SceneComponent Object Reference") (VisibleCustomer :type Integer)))