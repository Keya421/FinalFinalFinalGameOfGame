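; BP_CraftingBench is an interactable crafting bench actor, filed under the restaurant crafting assets, that opens the crafting menu.
; On Interact it creates a WB_craftingGUI widget, stores it on the player's BP_ThirdPersonCharacter as CraftWidget and adds it to the viewport.
; It then switches the local player to UI-only input focused on the widget and shows the mouse cursor.
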(event `/Game/Hearthvale/Blueprint/PlayerData/BPI_Interact.Interact`
  (bind _returnvalue (`GameplayStatics.GetPlayerController` 0))
  (bind _returnvalue_2 (`|CreateWidget` "/Game/Hearthvale/Blueprint/UI/Crafting/WB_craftingGUI.WB_craftingGUI_C" _returnvalue))
  (set `/Game/ThirdPerson/Blueprints/BP_ThirdPersonCharacter.CraftWidget` _returnvalue_2 (cast `/Game/ThirdPerson/Blueprints/BP_ThirdPersonCharacter` (`GameplayStatics.GetPlayerPawn` 0) :!pure true))
  (`UserWidget.AddToViewport` _returnvalue_2 0)
  (`WidgetBlueprintLibrary.SetInputMode_UIOnlyEx` _returnvalue _returnvalue_2)
  (set `PlayerController.bShowMouseCursor` true _returnvalue))

(fn `UserConstructionScript`
  (`parent.UserConstructionScript`))