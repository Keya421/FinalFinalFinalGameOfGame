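; BP_FurnitureCheck is a footprint actor for restaurant furniture, apparently meant for testing placement overlaps.
; On BeginPlay or UpdatedCheck, after a tiny delay, it scales to the furniture's length and width and snaps to BPCRestaurantGrid.
; A downward visibility trace then drops it onto the ground, printing debug messages on a miss.
; The overlap validation is unfinished: CheckOverlap's logic is disconnected and UpdatedCheck's overlap loop does nothing.
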(event `UpdatedCheck`
  (`KismetSystemLibrary.Delay` 0.001)
  (`self.SetActorSize`)
  (for _ (`self.GetOverlappingComponents`)
    _))

(event `self.ReceiveBeginPlay`
  (`KismetSystemLibrary.Delay` 0.001)
  (`self.SetActorSize`))

(fn `CheckOverlap`
  (params (IgnoreActor :type "Array of Actor Object Reference"))
  (returns (NoOverlap :type Boolean))
  (locals (ActorOverlap :type "Array of PrimitiveComponent Object Reference") (NewLocalVar :type "Array of PrimitiveComponent Object Reference")))

(fn `SetActorSize`
  (bind _returnvalue (`self.K2_GetActorLocation`))
  (`self.SetActorScale3D` (`KismetMathLibrary.MakeVector` (`KismetMathLibrary.Conv_IntToDouble` (`self.FurnitureLength`)) (`KismetMathLibrary.Conv_IntToDouble` (`self.FurnitureWidth`)) 1.0))
  (`self.K2_SetActorLocation` (`/Game/Hearthvale/Blueprint/Restaurant/BPC_RestaurantGrid.Get Grid Location` (`self.BPC_RestaurantGrid`) (`self.K2_GetActorLocation`)))
  (bind _outhit (`KismetSystemLibrary.LineTraceSingle` _returnvalue (+ (* (* (`self.GetActorUpVector`) -1.0) 500.0) _returnvalue) "TraceTypeQuery1"))
  (bind (_bblockinghit _binitialoverlap _time _distance _location) (`GameplayStatics.BreakHitResult` _outhit))
  (if _bblockinghit
    (`self.K2_SetActorLocation` _location)
    (else
      (`KismetSystemLibrary.PrintString` "where the fuck are you?")
      (`KismetSystemLibrary.PrintString` "you're probably in the air, so i couldnt place it down to the ground."))))

(fn `UserConstructionScript`)