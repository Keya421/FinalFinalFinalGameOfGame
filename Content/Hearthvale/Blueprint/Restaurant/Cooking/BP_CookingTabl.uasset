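; BP_CookingTabl is the interactable cooking table in the restaurant, opening the cooking UI when used.
; ShowInteract sends a "Cooking Table" prompt, along with ChildInteract entries, to the player character's interact widget.
; Interact creates WBP_CookingUI, adds it to the viewport, switches input to UI-only and enables the mouse cursor through BP_ThirdPersonCharacter.
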(event `/Game/Hearthvale/Blueprint/PlayerData/BPI_Interact.Interact`
  (params (`Hit Component` :type "ActorComponent Object Reference"))
  (bind _returnvalue (`GameplayStatics.GetPlayerController` 0))
  (bind _returnvalue_2 (`|CreateWidget` "/Game/Hearthvale/Blueprint/UI/Cooking/WBP_CookingUI.WBP_CookingUI_C" _returnvalue))
  (`UserWidget.AddToViewport` _returnvalue_2 0)
  (`WidgetBlueprintLibrary.SetInputMode_UIOnlyEx` _returnvalue _returnvalue_2)
  (`/Game/ThirdPerson/Blueprints/BP_ThirdPersonCharacter.EnableShowMouse` (cast `/Game/ThirdPerson/Blueprints/BP_ThirdPersonCharacter` (`GameplayStatics.GetPlayerPawn` 0) :!pure true) true))

(event `/Game/Hearthvale/Blueprint/PlayerData/BPI_Interact.ShowInteract`
  (`/Game/ThirdPerson/Blueprints/BP_ThirdPersonCharacter.SetInteractWidget` (cast `/Game/ThirdPerson/Blueprints/BP_ThirdPersonCharacter` (`GameplayStatics.GetPlayerPawn` 0) :!pure true) (`|MakeArray` (make `/Game/Hearthvale/Blueprint/UI/Interact/ST_InteractSettings` "Cooking Table") (`self.ChildInteract`) (`self.ChildInteract2`)) self))

(fn `UserConstructionScript`
  (`parent.UserConstructionScript`))