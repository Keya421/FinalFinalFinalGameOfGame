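; Vendor spawner actor that places BP_Vendor at its own location in the evening once the vendor quest is finished.
; BeginPlay enables Tick only if the game instance flags the quest as finished.
; Tick reads Time from BP_WeatherSpawn, spawning above 18 on every tick without an existing-vendor check, and otherwise destroying one found vendor.
; ForceSpawn triggers the same spawn directly.
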(event `self.ReceiveBeginPlay`
  (if (`/Game/Hearthvale/Blueprint/GI_Hearthvale.bVendorQuestFinished` (cast `/Game/Hearthvale/Blueprint/GI_Hearthvale` (`GameplayStatics.GetGameInstance`) :!pure true))
    (`self.SetActorTickEnabled` true)
    (else
      (`self.SetActorTickEnabled` false))))

(event `ForceSpawn`
  (`|SpawnActorFromClass` "/Game/Hearthvale/Blueprint/Vendor/BP_Vendor.BP_Vendor_C" (`KismetMathLibrary.MakeTransform` (`self.K2_GetActorLocation`)) "Undefined" "MultiplyWithRoot" null null :!label _label))

(event `self.ReceiveTick`
  (params (DeltaSeconds :type "Float (single-precision)"))
  (`KismetSystemLibrary.PrintString` "VendorCheckSpawn")
  (bind _returnvalue (`GameplayStatics.GetActorOfClass` "/Game/Hearthvale/Blueprint/Weather/BP_WeatherSpawn.BP_WeatherSpawn_C"))
  (`/Engine/EditorBlueprintResources/StandardMacros.IsValid` _returnvalue
    (:`Is Valid`
      (if (> (`/Game/Hearthvale/Blueprint/Weather/BP_WeatherSpawn.Time` _returnvalue) 18.0)
        (goto _label)
        (else
          (bind _returnvalue_2 (`GameplayStatics.GetActorOfClass` "/Game/Hearthvale/Blueprint/Vendor/BP_Vendor.BP_Vendor_C"))
          (`/Engine/EditorBlueprintResources/StandardMacros.IsValid` _returnvalue_2
            (:`Is Valid`
              (`self.K2_DestroyActor` _returnvalue_2))))))))

(fn `UserConstructionScript`)