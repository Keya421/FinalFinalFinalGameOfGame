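; BP_Vendor is a vendor that opens a shop interface when the player interacts with it.
; Interact creates WBP_Vendor, adds it to the viewport, sets DisableMovement on the player's BP_ThirdPersonCharacter and shows the mouse cursor.
; Back re-enables movement and hides the cursor, but does not remove the widget itself.
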(event `/Game/Hearthvale/Blueprint/PlayerData/BPI_Interact.Interact`
  (params (`Hit Component` :type "ActorComponent Object Reference"))
  (bind _returnvalue (`GameplayStatics.GetPlayerController` 0))
  (bind _returnvalue_2 (`|CreateWidget` "/Game/Hearthvale/A/UI-AP/WBP_Vendor.WBP_Vendor_C" _returnvalue))
  (`UserWidget.AddToViewport` _returnvalue_2 0)
  (set `/Game/ThirdPerson/Blueprints/BP_ThirdPersonCharacter.DisableMovement` true (cast `/Game/ThirdPerson/Blueprints/BP_ThirdPersonCharacter` (`Controller.K2_GetPawn` _returnvalue) :!pure true))
  (set `PlayerController.bShowMouseCursor` true _returnvalue))

(event `Back`
  (bind _returnvalue (`GameplayStatics.GetPlayerController` 0))
  (bind _asbp_third_person_character (cast `/Game/ThirdPerson/Blueprints/BP_ThirdPersonCharacter` (`Controller.K2_GetPawn` _returnvalue)))
  (set `/Game/ThirdPerson/Blueprints/BP_ThirdPersonCharacter.DisableMovement` false _asbp_third_person_character)
  (set `PlayerController.bShowMouseCursor` false _returnvalue))

(fn `UserConstructionScript`)