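; Farming plot where the player plants seeds from the selected hotbar slot and harvests the grown crop into the inventory.
; Plant either harvests or starts growth, spawning the seed data's crop actor and consuming the seed.
; A looping timer stretches the crop's Z scale per stage until harvestable; harvest never resets GrowthStage.
; A box overlap shows the Cube while the player is inside.
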(event `startGrow`
  (bind _asbp_third_person_character (cast `/Game/ThirdPerson/Blueprints/BP_ThirdPersonCharacter` (`GameplayStatics.GetPlayerCharacter` 0) :!pure true))
  (bind _itemdata (`/Game/Kristian/inventory/WBP_ItemSlot.itemData` (`|GetArrayItem` (`/Game/Kristian/inventory/WBP_inventory.HotbarArray` (`/Game/ThirdPerson/Blueprints/BP_ThirdPersonCharacter.InventoryWidget` _asbp_third_person_character)) (- (`/Game/ThirdPerson/Blueprints/BP_ThirdPersonCharacter.SelectedSlot` _asbp_third_person_character) 1))))
  (bind (_actorclass _cropdata) (defaults `Object` (castclass `/Game/Hearthvale/Blueprint/Items/ItemData/Farming/Seeds/DA_FarmingSeeds` (`.ItemClass_20_04EDF3F8416E8B472A41CC8E06E4FB6F` (break `/Game/Kristian/inventory/ST_items` _itemdata)) :!pure true)))
  (bind _returnvalue (`KismetSystemLibrary.K2_SetTimerDelegate` (delegate `Growing`) 5.0 true))
  (set `self.timerRef` _returnvalue)
  (set `self.IsGrowing` true)
  (bind _returnvalue_2 (`|SpawnActorFromClass` _actorclass (`KismetMathLibrary.Conv_VectorToTransform` (`SceneComponent.K2_GetComponentLocation` (`self.Scene`))) "Undefined" "MultiplyWithRoot" null null))
  (set `self.CropRef` _returnvalue_2)
  (set `self.Crop Data` _cropdata)
  (`/Game/ThirdPerson/Blueprints/BP_ThirdPersonCharacter.RemoveInventoryItem` (cast `/Game/ThirdPerson/Blueprints/BP_ThirdPersonCharacter` (`GameplayStatics.GetPlayerCharacter` 0) :!pure true) _itemdata))

(event `plant`
  (bind _asbp_third_person_character (cast `/Game/ThirdPerson/Blueprints/BP_ThirdPersonCharacter` (`GameplayStatics.GetPlayerCharacter` 0) :!pure true))
  (if (`self.Isharvestable`)
    (`self.Harvest`)
    (elif (`self.IsGrowing`)
      _
      (elif (`.bSuccess` (castclass `/Game/Hearthvale/Blueprint/Items/ItemData/Farming/Seeds/DA_FarmingSeeds` (`.ItemClass_20_04EDF3F8416E8B472A41CC8E06E4FB6F` (break `/Game/Kristian/inventory/ST_items` (`/Game/Kristian/inventory/WBP_ItemSlot.itemData` (`|GetArrayItem` (`/Game/Kristian/inventory/WBP_inventory.HotbarArray` (`/Game/ThirdPerson/Blueprints/BP_ThirdPersonCharacter.InventoryWidget` _asbp_third_person_character)) (- (`/Game/ThirdPerson/Blueprints/BP_ThirdPersonCharacter.SelectedSlot` _asbp_third_person_character) 1))))) :!pure true))
        (`self.startGrow`)))))

(event `Growing`
  (bind _growthstage (`self.growthStage`))
  (bind _cropref (`self.CropRef`))
  (bind (_returnvalue_x _returnvalue_y) (`KismetMathLibrary.BreakVector` (`self.GetActorScale3D` _cropref)))
  (bind _result (`/Engine/EditorBlueprintResources/StandardMacros.IncrementInt` _growthstage)
    (:`  `
      (`self.SetActorScale3D` _cropref (`KismetMathLibrary.MakeVector` _returnvalue_x _returnvalue_y (* 1.0 _growthstage)))
      (if (>= _result 3)
        (`KismetSystemLibrary.K2_PauseTimerHandle` (`self.timerRef`))
        (set `self.IsGrowing` false)
        (set `self.Isharvestable` true)))))

(event `Harvest`
  (`self.K2_DestroyActor` (`self.CropRef`))
  (bind _asbp_third_person_character (cast `/Game/ThirdPerson/Blueprints/BP_ThirdPersonCharacter` (`GameplayStatics.GetPlayerCharacter` 0)))
  (`/Game/ThirdPerson/Blueprints/BP_ThirdPersonCharacter.AddInventoryItem` _asbp_third_person_character (`self.Crop Data`) 1)
  (set `self.Isharvestable` false))

(event `self.Box.OnComponentBeginOverlap`
  (params (OverlappedComponent :type "PrimitiveComponent Object Reference") (OtherActor :type "Actor Object Reference") (OtherComp :type "PrimitiveComponent Object Reference") (OtherBodyIndex :type Integer) (bFromSweep :type Boolean) (SweepResult :type "HitResult Structure (by ref)"))
  (bind _asbp_third_person_character (cast `/Game/ThirdPerson/Blueprints/BP_ThirdPersonCharacter` OtherActor))
  (`/Engine/EditorBlueprintResources/StandardMacros.IsValid` _asbp_third_person_character
    (:`Is Valid`
      (`SceneComponent.SetVisibility` (`self.Cube`) true false))))

(event `self.Box.OnComponentEndOverlap`
  (params (OverlappedComponent :type "PrimitiveComponent Object Reference") (OtherActor :type "Actor Object Reference") (OtherComp :type "PrimitiveComponent Object Reference") (OtherBodyIndex :type Integer))
  (bind _asbp_third_person_character (cast `/Game/ThirdPerson/Blueprints/BP_ThirdPersonCharacter` OtherActor))
  (`/Engine/EditorBlueprintResources/StandardMacros.IsValid` _asbp_third_person_character
    (:`Is Valid`
      (`SceneComponent.SetVisibility` (`self.Cube`) false false))))

(fn `UserConstructionScript`)