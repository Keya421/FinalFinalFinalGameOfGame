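; Anim notify for footsteps that plays a surface-specific sound and counts steps.
; On notify, it traces down from the mesh owner and switches on the hit surface type for grass, marble or dirt, playing the sound at world origin rather than at the hit.
; Each match increments and prints Steps1 on the player's BP_ThirdPersonCharacter, whichever mesh fired it.
; A separate Sound function plays only the marble sound.
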(fn `Received_Notify`
  (params (MeshComp :type "SkeletalMeshComponent Object Reference") (Animation :type "AnimSequenceBase Object Reference") (EventReference :type "AnimNotifyEventReference Structure (by ref)"))
  (returns (ReturnValue :type Boolean))
  (bind _returnvalue (`ActorComponent.GetOwner` MeshComp))
  (bind _returnvalue_2 (`Actor.K2_GetActorLocation` _returnvalue))
  (bind (_outhit _returnvalue_3) (`KismetSystemLibrary.LineTraceSingle` :`Start` _returnvalue_2 :`End` (+ _returnvalue_2 (* (`Actor.GetActorUpVector` _returnvalue) -200.0)) :`TraceChannel` "TraceTypeQuery1" :`DrawDebugType` "ForDuration"))
  (if _returnvalue_3
    (switch `EPhysicalSurface` (`GameplayStatics.GetSurfaceType` _outhit)
      (:`SurfaceType1`
        (`GameplayStatics.PlaySoundAtLocation` "/Game/Hearthvale/A/SOUNDS-AP/FootstepsGrass.FootstepsGrass" (0.0 0.0 0.0) (struct) 0.5 1.0 0.0 null null null null))
      (:`SurfaceType2`
        (`GameplayStatics.PlaySoundAtLocation` "/Game/Hearthvale/A/SOUNDS-AP/FootstepsMarble.FootstepsMarble" (0.0 0.0 0.0) (struct) 0.5 1.0 0.0 null null null null))
      (:`SurfaceType3`
        (`GameplayStatics.PlaySoundAtLocation` "/Game/Hearthvale/A/SOUNDS-AP/FootstepsDirt.FootstepsDirt" (0.0 0.0 0.0) (struct) 0.5 1.0 0.0 null null null null)))
    (bind _asbp_third_person_character (cast `/Game/ThirdPerson/Blueprints/BP_ThirdPersonCharacter` (`GameplayStatics.GetPlayerPawn` 0)))
    (bind _output_get (set `/Game/ThirdPerson/Blueprints/BP_ThirdPersonCharacter.steps1` (+ (`/Game/ThirdPerson/Blueprints/BP_ThirdPersonCharacter.steps1` _asbp_third_person_character) 1) _asbp_third_person_character))
    (`KismetSystemLibrary.PrintString` (`KismetStringLibrary.Conv_IntToString` _output_get))
    (return false)))

(fn `Sound`
  (`GameplayStatics.PlaySoundAtLocation` "/Game/Hearthvale/A/SOUNDS-AP/FootstepsMarble.FootstepsMarble" (0.0 0.0 0.0) (struct) 5.0 1.0 0.0 null null null null)
  (return))